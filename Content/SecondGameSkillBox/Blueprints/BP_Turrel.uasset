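; BP_Turrel is a turret that sweeps for the third-person player character and fires on it when spotted.
; In Patrol, a self-restarting timeline swings the gun back and forth across 180 degrees of yaw while Tick runs a forward sphere trace.
; Detection switches to Shoot, which turns the gun toward the player and starts a looping timer for line-trace hitscan shots with sound and damage.
; Losing the player clears the timer and resumes patrol.
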(event Custom|StartPatrol
  (bind _newtrack_0 (Timeline|Timeline PlayFromStart)
    (:Update
      (Transformation|SetWorldRotation (Variables|Default|GetGun) (Math|Rotator|Lerp(Rotator) (Variables|Default|GetCurrentRotation) (Variables|Default|GetTargetRotation) _newtrack_0) false false))
    (:Finished
      (switch Utilities|FlowControl|Switch|SwitchonETimelineDirection (Variables|Default|GetDirectionMove)
        (:Forward
          (Variables|Default|SetDirectionMove "Backward")
          (Variables|Default|SetTargetRotation (Variables|Default|GetStartRotation))
          (Variables|Default|SetCurrentRotation (Variables|Default|GetEndRotation)))
        (:Backward
          (Variables|Default|SetDirectionMove "Forward")
          (Variables|Default|SetTargetRotation (Variables|Default|GetEndRotation))
          (Variables|Default|SetCurrentRotation (Variables|Default|GetStartRotation))))
      (CallFunction|StartPatrol))))

(event Custom|StopTimeline
  (bind _newtrack_0 (Timeline|Timeline Stop)
    (:Update
      (Transformation|SetWorldRotation (Variables|Default|GetGun) (Math|Rotator|Lerp(Rotator) (Variables|Default|GetCurrentRotation) (Variables|Default|GetTargetRotation) _newtrack_0) false false))
    (:Finished
      (switch Utilities|FlowControl|Switch|SwitchonETimelineDirection (Variables|Default|GetDirectionMove)
        (:Forward
          (Variables|Default|SetDirectionMove "Backward")
          (Variables|Default|SetTargetRotation (Variables|Default|GetStartRotation))
          (Variables|Default|SetCurrentRotation (Variables|Default|GetEndRotation)))
        (:Backward
          (Variables|Default|SetDirectionMove "Forward")
          (Variables|Default|SetTargetRotation (Variables|Default|GetEndRotation))
          (Variables|Default|SetCurrentRotation (Variables|Default|GetStartRotation))))
      (CallFunction|StartPatrol))))

(event Custom|Shooting
  (bind _isshoot (CallFunction|Shoot))
  (if _isshoot
    (bind _asbp_third_person_character (Utilities|Casting|CastToBP_ThirdPersonCharacter (Game|GetPlayerCharacter 0)))
    (Game|Damage|ApplyDamage _asbp_third_person_character 1e+01 0 0)))

(event Custom|StartShoot
  (CallFunction|Shoot)
  (bind _returnvalue (Utilities|Time|SetTimerbyEvent (EventDispatchers|CreateEvent :!event Custom|Shooting) 0.5 true))
  (Variables|Default|SetShootTimer _returnvalue))

(event EventBeginPlay
  (bind _gun (Variables|Default|GetGun))
  (bind _returnvalue (Transformation|GetWorldRotation _gun))
  (bind _output_get (Variables|Default|SetStartRotation _returnvalue))
  (bind _output_get_2 (Variables|Default|SetEndRotation (Math|Rotator|MakeRotator (.roll _output_get) (.pitch _output_get) (+ (.yaw _output_get) 1.8e+02))))
  (Variables|Default|SetCurrentRotation _returnvalue)
  (Variables|Default|SetTargetRotation _output_get_2)
  (CallFunction|StartPatrol))

(event EventTick
  (params (DeltaSeconds :type Float%20%28single-precision%29))
  (bind _gun (Variables|Default|GetGun))
  (bind _returnvalue (Transformation|GetWorldRotation _gun))
  (switch Utilities|FlowControl|Switch|SwitchonE_TurrelStates (Variables|Default|GetCurrentState)
    (:NewEnumerator0
      (bind _is_player_find (CallFunction|PlayerSearch))
      (if _is_player_find
        (Variables|Default|SetCurrentState "NewEnumerator1")
        (CallFunction|StopTimeline)))
    (:NewEnumerator1
      (Transformation|SetWorldRotation (Variables|Default|GetGun) (Math|Interpolation|RInterpTo (Math|Rotator|MakeRotator (.roll _returnvalue) (.pitch _returnvalue) (.yaw _returnvalue)) (Math|Rotator|MakeRotator (.roll _returnvalue) (.pitch _returnvalue) (- (.yaw (Math|Rotator|FindLookatRotation (Transformation|GetWorldLocation (Variables|Default|GetGun)) (Transformation|GetActorLocation (Game|GetPlayerCharacter 0)))) 9e+01)) (Utilities|Time|GetWorldDeltaSeconds) 0.0) false false)
      (Utilities|FlowControl|Sequence
        (:then_0
          (if (not (Variables|Default|GetbIsStartShoot))
            (CallFunction|StartShoot)
            (Variables|Default|SetbIsStartShoot true)))
        (:then_1
          (bind _is_player_find_2 (CallFunction|PlayerSearch))
          (if (not _is_player_find_2)
            (Utilities|Time|ClearandInvalidateTimerbyHandle (Variables|Default|GetShootTimer))
            (Variables|Default|SetbIsStartShoot false)
            (Variables|Default|SetCurrentState "NewEnumerator0")
            (switch Utilities|FlowControl|Switch|SwitchonETimelineDirection (Variables|Default|GetDirectionMove)
              (:Forward
                (Variables|Default|SetDirectionMove "Forward")
                (Variables|Default|SetTargetRotation (Variables|Default|GetEndRotation))
                (Variables|Default|SetCurrentRotation (Transformation|GetWorldRotation (Variables|Default|GetGun))))
              (:Backward
                (Variables|Default|SetDirectionMove "Backward")
                (Variables|Default|SetTargetRotation (Variables|Default|GetStartRotation))
                (Variables|Default|SetCurrentRotation (Transformation|GetWorldRotation (Variables|Default|GetGun)))))
            (CallFunction|StartPatrol)))))))

(fn ConstructionScript)

(fn PlayerSearch
  (bind _scene (Variables|Default|GetScene))
  (bind _returnvalue (Transformation|GetWorldLocation _scene))
  (bind (_outhit _returnvalue_2) (Collision|SphereTraceByChannel _returnvalue (+ _returnvalue (* (Math|Vector|GetForwardVector _scene) (Variables|Default|GetSearchDistance))) 1e+01 "TraceTypeQuery3" false 0 "ForOneFrame"))
  (if _returnvalue_2
    (Utilities|Casting|CastToBP_ThirdPersonCharacter (.HitActor (Collision|BreakHitResult _outhit))
      (:then
        (return true))
      (:CastFailed
        (return false)))
    (else
      (return false))))

(fn Shoot
  (bind _scene (Variables|Default|GetScene))
  (bind _returnvalue (Transformation|GetWorldLocation _scene))
  (bind (_outhit _returnvalue_2) (Collision|LineTraceByChannel _returnvalue (+ _returnvalue (* (Math|Vector|GetForwardVector _scene) (Variables|Default|GetShootDistance))) "TraceTypeQuery3" false 0 "None"))
  (if _returnvalue_2
    (Utilities|Casting|CastToBP_ThirdPersonCharacter (.HitActor (Collision|BreakHitResult _outhit))
      (:then
        (Audio|SpawnSoundatLocation "/Game/FPWeapon/Audio/FirstPersonTemplateWeaponFire02.FirstPersonTemplateWeaponFire02" (Transformation|GetActorLocation) "0, 0, 0" 1.0 1.0 0.0 0 0)
        (return true))
      (:CastFailed
        (return false)))
    (else
      (return false))))