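; BP_Door is a door actor that swings 90 degrees on Interact, with a gate that the Control event opens.
; BeginPlay stores the starting yaw as the base rotation.
; When the gate passes Interact, a FlipFlop alternates between playing and reversing a timeline that lerps the yaw between that base and minus 90 degrees from it.
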(event EventInteract
  (bind _currentrotation (Variables|Default|GetCurrentRotation))
  (Utilities|FlowControl|Gate true
    (:Exit
      (Utilities|FlowControl|FlipFlop
        (:A
          (bind _newtrack_0 (Timeline|Timeline Play)
            (:Update
              (Transformation|SetActorRotation (Math|Rotator|MakeRotator 0.0 0.0 (Math|Float|Lerp _currentrotation (+ _currentrotation -9e+01) _newtrack_0))))))
        (:B
          (Timeline|Timeline Reverse))))))

(event EventControl
  (bind _currentrotation (Variables|Default|GetCurrentRotation))
  (Utilities|FlowControl|Gate true) ; enters at Open
)

(event EventBeginPlay
  (Variables|Default|SetCurrentRotation (.yaw (Transformation|GetActorRotation))))

(fn ConstructionScript
  (|CallParentFunction))